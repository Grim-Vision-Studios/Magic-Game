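; BP_ProjectBase is a base projectile actor that flies toward an optional target and reports what it hits.
; The construction script configures ProjectileMovement from speed and gravity variables, enabling homing on the target's root when requested.
; On BeginPlay it ignores its instigator, or owner as fallback, and aims velocity at any valid target.
; A box collision hit calls OnProjectHit, spawns impact effect and sound, then destroys the actor.
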(event OnComponentHit(BoxCollision)
  (params (HitComponent :type Primitive%20Component%20Object%20Reference) (OtherActor :type Actor%20Object%20Reference) (OtherComp :type Primitive%20Component%20Object%20Reference) (NormalImpulse :type Vector :default "0, 0, 0") (Hit :type Hit%20Result%20Structure%20%28by%20ref%29))
  (bind _location (Collision|BreakHitResult Hit))
  ;[1 1 1] On Hit of enemy and what happens
  (Default|CallOnProjectHit OtherActor Hit)
  (Effects|SpawnEmitteratLocation (Variables|Effects|GetImpact%20Effect) _location "0.000000,0.000000,50.000000")
  (Audio|PlaySoundatLocation (Variables|Sounds|GetInpact%20Sound) _location "0, 0, 0" 0.2 1.0 0.1 0 0 0 0)
  (Actor|DestroyActor))

(event Custom|Rotate%20To%20Target
  ;[1 1 1] Find Target
  (Variables|/Script/Engine.MovementComponent|SetVelocity (Variables|Default|GetProjectileMovement) (* (Math|Vector|GetUnitDirection(Vector) (Transformation|GetActorLocation) (Transformation|GetActorLocation (Variables|Target|GetTarget))) (Variables|ProjectSettings|GetSpeed))))

(event EventBeginPlay
  (bind _returnvalue (Game|GetInstigator))
  ;[1 1 1] Spawn attack in game
  (Collision|IgnoreActorwhenMoving (Variables|Default|GetBoxCollision) (select (Utilities|IsValid _returnvalue) _returnvalue (Components|GetOwner)) true)
  (Variables|Target|GetTarget
    (:then
      (CallFunction|RotatetoTarget))
    (:else)))

(fn ConstructionScript
  (bind _projectilemovement (Variables|Default|GetProjectileMovement))
  (Variables|/Script/Engine.ProjectileMovementComponent|SetInitialSpeed _projectilemovement (Variables|ProjectSettings|GetSpeed))
  (Variables|/Script/Engine.ProjectileMovementComponent|SetMaxSpeed _projectilemovement (Variables|ProjectSettings|GetSpeed))
  (Variables|/Script/Engine.ProjectileMovementComponent|SetProjectileGravityScale _projectilemovement (Variables|ProjectSettings|GetGravity))
  (Variables|Target|GetTarget
    (:then
      (if (Variables|ProjectSettings|GetIsHoming)
        (Variables|/Script/Engine.ProjectileMovementComponent|SetbIsHomingProjectile _projectilemovement true)
        (Variables|/Script/Engine.ProjectileMovementComponent|SetHomingTargetComponent _projectilemovement (Variables|/Script/Engine.Actor|GetRootComponent (Variables|Target|GetTarget)))))
    (:else)))