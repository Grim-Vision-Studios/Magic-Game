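; Lightning strike area-of-effect actor that shows a ground warning decal before it strikes.
; On BeginPlay it attempts to snap to the floor under AttackTarget, spawns an energy-beam decal, waits DelayBeforeStrike, calls Trigger, then destroys the decal.
; The floor trace uses the target's location as both start and end (end multiplied by one), so it has zero length rather than reaching downward.
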(event Custom|MoveToFloor
  ;[1 1 1] Move Decal to floor
  (bind _attacktarget (Variables|Default|GetAttackTarget)
    (:then
      (bind (_outhit _returnvalue) (Collision|LineTraceByChannel (Transformation|GetActorLocation _attacktarget) (* (Transformation|GetActorLocation _attacktarget) "1.000000,1.000000,1.000000") "TraceTypeQuery1" false (Utilities|Array|MakeArray _attacktarget) "ForDuration" false))
      (if _returnvalue
        (Transformation|SetActorLocation (.ImpactPoint (Collision|BreakHitResult _outhit)) true false)))
    (:else)))

(event EventBeginPlay
  (|CallParentFunction)
  (CallFunction|MovetoFloor)
  (bind _returnvalue (Rendering|Decal|SpawnDecalatLocation "/Game/RPGEffects/Materials/M_EnergyBeam.M_EnergyBeam" "25.000000,256.000000,256.000000" (Transformation|GetActorLocation) "-90.000000,0.000000,0.000000" 0.0))
  (Utilities|FlowControl|Delay (Variables|Default|GetDelay%20before%20Strike))
  (CallFunction|Trigger)
  (Utilities|IsValid _returnvalue
    (:Is%20Valid
      (Components|DestroyComponent _returnvalue))))

(event Collision|EventActorBeginOverlap
  (params (OtherActor :type Actor%20Object%20Reference))
  (|CallParentFunction OtherActor) ; This node is disabled and will not be called.\nDrag off pins to build functionality.
)

(event EventTick
  (params (DeltaSeconds :type Float%20%28single-precision%29))
  (|CallParentFunction DeltaSeconds) ; This node is disabled and will not be called.\nDrag off pins to build functionality.
)

(fn ConstructionScript
  (|CallParentFunction))