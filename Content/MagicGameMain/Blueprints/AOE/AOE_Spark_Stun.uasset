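; AOE spark stun effect actor that briefly stuns BP_Enemy actors overlapping its Sphere component.
; On overlap it disables the enemy's movement, plays a dizzy animation, waits two seconds, then restores walking and destroys itself.
; A single Delay serves all overlaps, so only the most recently overlapped enemy gets walking restored.
; Trigger only forwards to the parent class.
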(event OnComponentBeginOverlap(Sphere)
  (params (OverlappedComponent :type Primitive%20Component%20Object%20Reference) (OtherActor :type Actor%20Object%20Reference) (OtherComp :type Primitive%20Component%20Object%20Reference) (OtherBodyIndex :type Integer) (bFromSweep :type Boolean) (SweepResult :type Hit%20Result%20Structure%20%28by%20ref%29))
  ;[1 1 1] On overlap stun AI
  (bind _asbp_enemy (Utilities|Casting|CastToBP_Enemy OtherActor))
  (Pawn|Components|CharacterMovement|DisableMovement (Variables|/Script/Engine.Character|GetCharacterMovement _asbp_enemy))
  (Components|Animation|PlayAnimation (Variables|/Script/Engine.Character|GetMesh _asbp_enemy) "/Game/BattleWizardPolyart/Animations/DizzyAnim.DizzyAnim" false)
  (Utilities|FlowControl|Delay 2.0)
  (Pawn|Components|CharacterMovement|SetMovementMode (Variables|/Script/Engine.Character|GetCharacterMovement _asbp_enemy) "MOVE_Walking" 0)
  (Actor|DestroyActor))

(event Collision|EventActorBeginOverlap
  (params (OtherActor :type Actor%20Object%20Reference)))

(event EventTick
  (params (DeltaSeconds :type Float%20%28single-precision%29)))

(event EventTrigger
  (|CallParentFunction))

(event EventBeginPlay
  (|CallParentFunction) ; This node is disabled and will not be called.\nDrag off pins to build functionality.
)

(fn ConstructionScript
  (|CallParentFunction))