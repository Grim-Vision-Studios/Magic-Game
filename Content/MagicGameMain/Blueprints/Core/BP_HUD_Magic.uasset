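; BP_HUD_Magic is the HUD Blueprint that puts the player's main HUD widget on screen.
; On BeginPlay it creates W_PlayerHud for the owning player controller, stores it and adds it to the viewport.
; LinkOwnerSkillHolder then hands the controlled pawn's BP_AC_SkillHolder component to the widget's skill hotbar, if that component is valid.
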(event Custom|LinkOwnerSkillHolder
  (bind _returnvalue (Game|Player|GetOwningPlayerController))
  (bind _returnvalue_2 (Pawn|GetControlledPawn _returnvalue))
  (bind _returnvalue_3 (Actor|GetComponentbyClass _returnvalue_2 "/Game/MagicGameMain/Blueprints/Systems/Skills/BP_AC_SkillHolder.BP_AC_SkillHolder_C"))
  (Utilities|IsValid _returnvalue_3
    (:Is%20Valid
      (Default|SetLinkedSkillHolder (Variables|/Game/MagicGameMain/Blueprints/Widgets/W_PlayerHud.W_PlayerHud_C|GetW_SkillHotbar (Variables|Default|GetHud%20Widget)) _returnvalue_3))))

(event EventBeginPlay
  (bind _returnvalue (UserInterface|CreateWidget "/Game/MagicGameMain/Blueprints/Widgets/W_PlayerHud.W_PlayerHud_C" (Game|Player|GetOwningPlayerController)))
  (bind _output_get (Variables|Default|SetHud%20Widget _returnvalue))
  (UserInterface|Viewport|AddtoViewport _output_get 0)
  (CallFunction|LinkOwnerSkillHolder))

(fn ConstructionScript)