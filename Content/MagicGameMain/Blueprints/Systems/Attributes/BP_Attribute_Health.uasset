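; Health attribute that applies incoming damage to the actor that owns it and signals hits and death.
; On Init it casts its outer object to an Actor, stores it as the owner and binds to that actor's OnTakeAnyDamage.
; Each damage event decreases the current value, then calls OnDeath if the value is empty, otherwise OnHit with the damage type.
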(event Custom|OnTakeAnyDamage_Event
  (params (DamagedActor :type Actor%20Object%20Reference) (Damage :type Float%20%28single-precision%29) (DamageType :type Damage%20Type%20Object%20Reference) (InstigatedBy :type Controller%20Object%20Reference) (DamageCauser :type Actor%20Object%20Reference))
  (CallFunction|DecreaseCurrentValue Damage)
  (if (CallFunction|IsEmpty)
    (Default|CallOnDeath)
    (else
      (Default|CallOnHit DamageType))))

(event EventInit
  (bind _asactor (Utilities|Casting|CastToActor (Utilities|GetOuterObject self)))
  (bind _output_get (Variables|Default|SetOwner _asactor))
  (EventDispatchers|AssignOnTakeAnyDamage _output_get (delegate Custom|OnTakeAnyDamage_Event)))