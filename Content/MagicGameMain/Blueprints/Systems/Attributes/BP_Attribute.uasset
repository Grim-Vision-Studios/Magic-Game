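; BP_Attribute is a generic attribute that holds a current value between zero and a maximum, with getters for both.
; Increase and decrease functions route through a clamped setter that records the previous value, then fire their matching dispatchers.
; CurrentValue uses a RepNotify to broadcast a value-changed dispatcher.
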(fn GetMaxValue
  (return (Variables|Default|GetMaxValue)))

(fn GetCurrentValue
  (return (Variables|Default|GetCurrentValue)))

(fn IncreaseValue
  (params (Increase :type Float%20%28double-precision%29))
  (CallFunction|SetCurrentValue (+ (Variables|Default|GetCurrentValue) Increase))
  (Default|CallOnValueIncrease))

(fn DecreaseValue
  (params (Decrease :type Float%20%28double-precision%29))
  (CallFunction|SetCurrentValue (- (Variables|Default|GetCurrentValue) Decrease))
  (Default|CallOnValueDecrease))

(fn SetCurrentValue
  (params (NewCurrentValue :type Float%20%28double-precision%29))
  (LocalVariables|SetPreviousValue (Variables|Default|GetCurrentValue))
  (Variables|Default|SetCurrentValue (Math|Float|Clamp(Float) NewCurrentValue 0.0 (Variables|Default|GetMaxValue))))

(fn OnRepCurrentValue
  (Default|CallOnCurrentValueChanged))