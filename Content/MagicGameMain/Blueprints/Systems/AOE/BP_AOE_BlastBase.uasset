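; Base blast area-of-effect actor that layers sound, visual effect and radial damage onto its parent AOE class.
; Trigger runs the parent logic, then spawns the attached blast effect and plays the blast sound at the actor's location.
; Hit applies full, non-falloff radial damage around the hit location.
; The actor destroys itself when the effect finishes, or after a short delay if no effect is set.
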(event Custom|CustomEvent
  (params (PSystem :type Niagara%20Component%20Object%20Reference))
  ;[1 1 1] Blast Effect
  (Actor|DestroyActor))

(event Custom|spawnBlastEffect
  ;[1 1 1] Blast Effect
  (bind _blast_effect (Variables|Default|GetBlast%20Effect)
    (:then
      (bind _returnvalue (Niagara|SpawnSystemAttached _blast_effect (Variables|Default|GetDefaultSceneRoot) "None" (Transformation|GetActorLocation) "0, 0, 0" "KeepRelativeOffset" false))
      (EventDispatchers|BindEventtoOnSystemFinished _returnvalue (delegate Custom|CustomEvent)))
    (:else
      (Utilities|FlowControl|Delay 1.0)
      (Actor|DestroyActor))))

(event Custom|PlayBlastSound
  ;[1 1 1] Blast Sounds
  (bind _blast_sound (Variables|Default|GetBlast%20sound)
    (:then
      (Audio|PlaySoundatLocation _blast_sound (Transformation|GetActorLocation) "0, 0, 0" 1.0 1.0 0.0 0 0 0 0))
    (:else)))

(event EventBeginPlay
  (|CallParentFunction) ; This node is disabled and will not be called.\nDrag off pins to build functionality.
)

(event Collision|EventActorBeginOverlap
  (params (OtherActor :type Actor%20Object%20Reference)))

(event EventTick
  (params (DeltaSeconds :type Float%20%28single-precision%29)))

(event Collision|EventHit
  (params (MyComp :type Primitive%20Component%20Object%20Reference) (Other :type Actor%20Object%20Reference) (OtherComp :type Primitive%20Component%20Object%20Reference) (bSelfMoved :type Boolean) (HitLocation :type Vector :default "0, 0, 0") (HitNormal :type Vector :default "0, 0, 0") (NormalImpulse :type Vector :default "0, 0, 0") (Hit :type Hit%20Result%20Structure%20%28by%20ref%29))
  (Game|Damage|ApplyRadialDamage 1e+02 HitLocation 5e+02 0 0 self 0 true "ECC_WorldStatic"))

(event EventSpawnAOESphere
  (|CallParentFunction))

(event EventTrigger
  (|CallParentFunction)
  (CallFunction|SpawnBlastEffect)
  (CallFunction|PlayBlastSound))

(fn ConstructionScript
  (|CallParentFunction))