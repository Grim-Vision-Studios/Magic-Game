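; BP_AC_SkillHolder is a component that holds its owner's skill slots.
; On BeginPlay it rebuilds the slots from SkillSetup, creating a BP_SkillDataObject per row with the row name and slot index, then signals initialization.
; Skills can be set by index, which signals an update, or added to the first slot whose skill data is invalid, reporting failure when none is open.
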(event EventBeginPlay
  (CallFunction|InitSkillSlots))

(fn InitSkillSlots
  (Utilities|Array|Clear (Variables|Default|GetSkills))
  (for (_array_element _array_index) (Variables|Default|GetSkillSetup)
    (bind _returnvalue (Game|ConstructObjectfromClass (Components|GetOwner) "/Game/MagicGameMain/Blueprints/Systems/Skills/BP_SkillDataObject.BP_SkillDataObject_C" (.RowName (Utilities|Struct|BreakDataTableRowHandle _array_element)) _array_index))
    (Utilities|Array|Add (Variables|Default|GetSkills) _returnvalue))
  (Default|CallOnSkillsInit))

(fn GetSkills
  (return (Variables|Default|GetSkills)))

(fn SetSlotSkill
  (params (Index :type Integer) (NewSkill :type BP%20Skill%20Data%20Object%20Object%20Reference))
  (Utilities|Array|SetArrayElem (Variables|Default|GetSkills) Index NewSkill)
  (Default|CallOnSkillUpdated Index NewSkill))

(fn AddSkilltoOpenSlot
  (params (AddedSkill :type BP%20Skill%20Data%20Object%20Object%20Reference))
  (bind (_openslotfound _array_index) (CallFunction|GetFirstOpenSlot))
  (if _openslotfound
    (CallFunction|SetSlotSkill _array_index AddedSkill)
    (return true)
    (else
      (return false))))

(fn GetFirstOpenSlot
  (for (_array_element _array_index) (Variables|Default|GetSkills)
    (bind _isvailid (Default|GetSkillData _array_element))
    (if (not _isvailid)
      (return true _array_index)))
  (return false -1))