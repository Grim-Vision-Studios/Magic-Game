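; Skill handler component for the Heal skill, which drops a healing area on the ground beneath its owner.
; On use with a valid Target, it line-traces toward an endpoint made by scaling the owner's Z coordinate by -1000, ignoring Target.
; A hit spawns and triggers a timed AOE_HealBase there, whose overlap event sends a fixed heal message only to Target.
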(event Custom|OnHealTarget
  (params (Actor :type Actor%20Object%20Reference))
  (if (== Actor (Variables|Default|GetTarget))
    (Class|BPIDamageInterface|Heal(Message) Actor 1e+01)))

(event EventBeginPlay
  (|CallParentFunction) ; This node is disabled and will not be called.\nDrag off pins to build functionality.
)

(event EventTick
  (params (DeltaSeconds :type Float%20%28single-precision%29))
  (|CallParentFunction DeltaSeconds) ; This node is disabled and will not be called.\nDrag off pins to build functionality.
)

(event EventStartUse
  (bind _returnvalue (Components|GetOwner))
  (bind _target (Variables|Default|GetTarget))
  (bind _returnvalue_2 (Transformation|GetActorLocation _returnvalue))
  (Utilities|IsValid _target
    (:Is%20Valid
      (bind (_outhit _returnvalue_3) (Collision|LineTraceByChannel _returnvalue_2 (* _returnvalue_2 "1.000000,1.000000,-1000.000000") "TraceTypeQuery1" false (Utilities|Array|MakeArray _target) "None"))
      (if _returnvalue_3
        (bind _returnvalue_4 (Game|SpawnActorfromClass "/Game/MagicGameMain/Blueprints/Systems/AOE/AOE_HealBase.AOE_HealBase_C" (Math|Transform|MakeTransform (.Location (Collision|BreakHitResult _outhit)) "0, 0, 0" "1.000000,1.000000,1.000000") "Undefined" "MultiplyWithRoot" 0 1.0 1e+01 false true false 0))
        (EventDispatchers|BindEventtoOnAoeOverlapActor _returnvalue_4 (delegate Custom|OnHealTarget))
        (Default|Trigger _returnvalue_4)))))