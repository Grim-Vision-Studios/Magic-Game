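; BP_AC_Skill_RockStrike is a skill component that launches a rock attack from its owner.
; On use, it spawns BP_Rock at the owner's transform, passes it the target and binds to its hit event.
; On impact, it sends damage to the hit actor through a message call.
; It then makes noise at the impact point, louder when that call returns true.
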(event Custom|RockHit
  (params (Other%20Actor :type Actor%20Object%20Reference) (Hit :type Hit%20Result%20Structure))
  (bind _returnvalue (Components|GetOwner))
  (bind _impactpoint (Collision|BreakHitResult Hit))
  (bind _wasdamage (Class|BPIDamageInterface|TakeDamage(Message) Other%20Actor (Utilities|Struct|MakeS_Info (Variables|Default|GetDamage) "NewEnumerator2" "NewEnumerator1")))
  (if _wasdamage
    (Class|Actor|MakeNoise _returnvalue 0.5 0 _impactpoint 0.1 "None")
    (else
      (Class|Actor|MakeNoise _returnvalue 0.2 0 _impactpoint 0.1 "None"))))

(event EventBeginPlay
  (|CallParentFunction) ; This node is disabled and will not be called.\nDrag off pins to build functionality.
)

(event EventTick
  (params (DeltaSeconds :type Float%20%28single-precision%29))
  (|CallParentFunction DeltaSeconds) ; This node is disabled and will not be called.\nDrag off pins to build functionality.
)

(event EventStartUse
  (bind _returnvalue (Components|GetOwner))
  (bind _returnvalue_2 (Game|SpawnActorfromClass "/Game/MagicGameMain/Blueprints/Systems/Projectiles/BP_Rock.BP_Rock_C" (Transformation|GetActorTransform _returnvalue) "Undefined" "MultiplyWithRoot" _returnvalue 1.2e+03 1.0 (Variables|Default|GetTarget) false 0))
  (EventDispatchers|BindEventtoOnProjectHit _returnvalue_2 (delegate Custom|RockHit)))