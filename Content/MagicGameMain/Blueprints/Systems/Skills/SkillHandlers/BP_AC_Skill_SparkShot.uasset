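; Skill handler component for the Spark Shot skill, which fires a spark projectile that damages what it hits.
; On use it spawns BP_Sparks at the skill spawn transform, passing the target and instigator, and binds to the projectile's hit event.
; A hit sends a typed damage message to the struck actor and makes noise at the impact point, louder when that message returns true.
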(event Custom|DamageEnemy
  (params (Other%20Actor :type Actor%20Object%20Reference) (Hit :type Hit%20Result%20Structure))
  (bind _returnvalue (Components|GetOwner))
  (bind _impactpoint (Collision|BreakHitResult Hit))
  (bind _wasdamage (Class|BPIDamageInterface|TakeDamage(Message) Other%20Actor (Utilities|Struct|MakeS_Info 2.0 "NewEnumerator2" "NewEnumerator1")))
  (if _wasdamage
    (Class|Actor|MakeNoise _returnvalue 0.5 0 _impactpoint 0.0 "None")
    (else
      (Class|Actor|MakeNoise _returnvalue 0.2 0 _impactpoint 0.0 "None"))))

(event EventBeginPlay
  (|CallParentFunction) ; This node is disabled and will not be called.\nDrag off pins to build functionality.
)

(event EventTick
  (params (DeltaSeconds :type Float%20%28single-precision%29))
  (|CallParentFunction DeltaSeconds) ; This node is disabled and will not be called.\nDrag off pins to build functionality.
)

(event EventStartUse
  (bind _returnvalue (Game|SpawnActorfromClass "/Game/MagicGameMain/Blueprints/Systems/Projectiles/BP_Sparks.BP_Sparks_C" (CallFunction|GetSkillSpawnTransform) "Undefined" "MultiplyWithRoot" (Components|GetOwner) 1.3e+03 0.0 (Variables|Default|GetTarget) true (Variables|Default|GetOwnerPawn)))
  (EventDispatchers|BindEventtoOnProjectHit _returnvalue (delegate Custom|DamageEnemy)))