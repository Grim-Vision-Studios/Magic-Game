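; BP_AC_Skill is a skill component that appears to serve as a base, with empty StartUse and EndUse events.
; On BeginPlay it caches the owning Pawn and that pawn's CameraComponent.
; GetSkillSpawnTransform offsets the owner's location by SpawnForwardOffset along the camera's horizontal forward vector, left unnormalized, and takes pitch and yaw from the camera with zero roll.
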(event Custom|StartUse)

(event Custom|EndUse)

(event EventBeginPlay
  (bind _aspawn (Utilities|Casting|CastToPawn (Components|GetOwner)))
  (bind _output_get (Variables|Default|SetOwnerPawn _aspawn))
  (Variables|Default|SetOwnerCamera (Actor|GetComponentbyClass _output_get "/Script/Engine.CameraComponent")))

(event EventTick
  (params (DeltaSeconds :type Float%20%28single-precision%29)))

(fn GetSkillSpawnTransform
  (bind _ownercamera (Variables|Default|GetOwnerCamera))
  (bind _returnvalue (Math|Vector|GetForwardVector _ownercamera))
  (bind _returnvalue_2 (Transformation|GetWorldRotation _ownercamera))
  (return (Math|Transform|MakeTransform (+ (Transformation|GetActorLocation (Components|GetOwner)) (* (Math|Vector|MakeVector (.x _returnvalue) (.y _returnvalue) 0.0) (LocalVariables|GetSpawnForwardOffset))) (Math|Rotator|MakeRotator 0.0 (.pitch _returnvalue_2) (.yaw _returnvalue_2)) "1.000000,1.000000,1.000000")))