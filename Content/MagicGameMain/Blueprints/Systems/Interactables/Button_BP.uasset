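; Button_BP is a one-shot interactable button that opens the door paired with it.
; On Interact it swaps the cube's material, searches all Door_BP actors for the first DoorValue matching its ButtonValue, and calls OpenDoor on it.
; If ChangeCameraView is set, it blends the view to that door and disables player input for a few seconds, without restoring the view itself.
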(event OnComponentBeginOverlap(Box)
  (params (OverlappedComponent :type Primitive%20Component%20Object%20Reference) (OtherActor :type Actor%20Object%20Reference) (OtherComp :type Primitive%20Component%20Object%20Reference) (OtherBodyIndex :type Integer) (bFromSweep :type Boolean) (SweepResult :type Hit%20Result%20Structure%20%28by%20ref%29)))

(event EventBeginPlay)

(event Collision|EventActorBeginOverlap
  (params (OtherActor :type Actor%20Object%20Reference)))

(event EventTick
  (params (DeltaSeconds :type Float%20%28single-precision%29)))

(event EventInteract
  (params (Player :type BP%20Third%20Person%20Character%20Object%20Reference))
  (Utilities|FlowControl|DoOnce false
    (:Completed
      (Rendering|Material|SetMaterial (Variables|Default|GetCube) 0 "/Engine/VREditor/BasicMeshes/MI_Cube_03.MI_Cube_03")
      (bind _outactors (Actor|GetAllActorsOfClass "/Game/MagicGameMain/Blueprints/Systems/Interactables/Door_BP.Door_BP_C"))
      (bind _array_element (Utilities|Array|ForEachLoopwithBreak _outactors :!label _label)
        (:LoopBody
          (if (== (Variables|/Game/MagicGameMain/Blueprints/Systems/Interactables/Door_BP.Door_BP_C|GetDoorValue _array_element) (Variables|Default|GetButtonValue))
            (Default|OpenDoor _array_element Player)
            (if (Variables|Default|GetChangeCameraView)
              (Game|Player|SetViewTargetwithBlend (Game|GetPlayerController 0) _array_element 0.1 "VTBlend_Linear" 0.0 false)
              (Input|DisableInput Player 0)
              (Utilities|FlowControl|Delay 3.5)
              (Input|EnableInput Player 0)
              (goto _label Break)
              (else
                (goto _label Break)))))))))

(fn ConstructionScript)