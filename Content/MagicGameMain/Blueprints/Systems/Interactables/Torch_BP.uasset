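; Torch interactable that lights when hit by a BP_Fire actor and opens a linked door.
; The fire effect starts deactivated and activates on a fire hit.
; A DoOnce then swaps the cube material and searches all Door_BP actors, calling OpenDoor on the first whose DoorValue matches this torch's ButtonValue.
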(event EventBeginPlay
  (Components|Activation|Deactivate (Variables|Default|GetP_Fire)))

(event Collision|EventActorBeginOverlap
  (params (OtherActor :type Actor%20Object%20Reference)))

(event EventTick
  (params (DeltaSeconds :type Float%20%28single-precision%29)))

(event Collision|EventHit
  (params (MyComp :type Primitive%20Component%20Object%20Reference) (Other :type Actor%20Object%20Reference) (OtherComp :type Primitive%20Component%20Object%20Reference) (bSelfMoved :type Boolean) (HitLocation :type Vector :default "0, 0, 0") (HitNormal :type Vector :default "0, 0, 0") (NormalImpulse :type Vector :default "0, 0, 0") (Hit :type Hit%20Result%20Structure%20%28by%20ref%29))
  (bind _asbp_fire (Utilities|Casting|CastToBP_Fire Other))
  (Components|Activation|Activate (Variables|Default|GetP_Fire) false)
  (Utilities|FlowControl|DoOnce false
    (:Completed
      (Rendering|Material|SetMaterial (Variables|Default|GetCube) 0 "/Engine/VREditor/BasicMeshes/MI_Cube_03.MI_Cube_03")
      (bind _outactors (Actor|GetAllActorsOfClass "/Game/MagicGameMain/Blueprints/Systems/Interactables/Door_BP.Door_BP_C"))
      (bind _array_element (Utilities|Array|ForEachLoopwithBreak _outactors :!label _label)
        (:LoopBody
          (if (== (Variables|/Game/MagicGameMain/Blueprints/Systems/Interactables/Door_BP.Door_BP_C|GetDoorValue _array_element) (Variables|Default|GetButtonValue))
            (Default|OpenDoor _array_element _asbp_fire)
            (goto _label Break)))))))

(fn ConstructionScript)