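; BP_Sparks is a spark projectile that plays an error buzz sound on spawn and creates a stun AOE on hit.
; The Hit event spawns AOE_Spark_Stun at the hit location, then immediately calls DestroyActor on that spawned actor.
; BeginPlay and overlap defer to the parent class; Tick is disabled and SpawnAOESphere is an empty stub.
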(event Collision|EventActorBeginOverlap
  (params (OtherActor :type Actor%20Object%20Reference))
  (|CallParentFunction OtherActor))

(event EventTick
  (params (DeltaSeconds :type Float%20%28single-precision%29))
  (|CallParentFunction DeltaSeconds) ; This node is disabled and will not be called.\nDrag off pins to build functionality.
)

(event EventBeginPlay
  (|CallParentFunction)
  (Audio|PlaySound2D "/Game/Interface_And_Item_Sounds/WAV/Error_Buzz_02.Error_Buzz_02" 1.0 1.0 0.0 0 0))

(event Collision|EventHit
  (params (MyComp :type Primitive%20Component%20Object%20Reference) (Other :type Actor%20Object%20Reference) (OtherComp :type Primitive%20Component%20Object%20Reference) (bSelfMoved :type Boolean) (HitLocation :type Vector :default "0, 0, 0") (HitNormal :type Vector :default "0, 0, 0") (NormalImpulse :type Vector :default "0, 0, 0") (Hit :type Hit%20Result%20Structure%20%28by%20ref%29))
  ;[1 1 1] Adding AOE to level
  (if true
    (bind _returnvalue (Game|SpawnActorfromClass "/Game/MagicGameMain/Blueprints/Systems/AOE/AOE_Spark_Stun.AOE_Spark_Stun_C" (Math|Conversions|ToTransform(Vector) HitLocation) "Undefined" "MultiplyWithRoot" 0 false true false 0))
    (Actor|DestroyActor _returnvalue)))

(fn ConstructionScript
  (|CallParentFunction))

(fn SpawnAOESphere)