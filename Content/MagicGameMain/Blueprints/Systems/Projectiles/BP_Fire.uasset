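; BP_Fire is a fire projectile that creates a short-lived area-of-effect fire when it hits a target.
; It extends a parent projectile's TargetHit event by spawning a fire AOE actor and destroying it after a brief delay.
; On BeginPlay, its box collision explicitly sets ignoring of the owner during movement to false.
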(event EventBeginPlay
  (|CallParentFunction)
  (Collision|IgnoreActorwhenMoving (Variables|Default|GetBoxCollision) (Components|GetOwner) false))

(event Collision|EventActorBeginOverlap
  (params (OtherActor :type Actor%20Object%20Reference))
  (|CallParentFunction OtherActor) ; This node is disabled and will not be called.\nDrag off pins to build functionality.
)

(event EventTick
  (params (DeltaSeconds :type Float%20%28single-precision%29))
  (|CallParentFunction DeltaSeconds) ; This node is disabled and will not be called.\nDrag off pins to build functionality.
)

(event EventTargetHit
  (params (Other%20Actor :type Actor%20Object%20Reference) (HitResult :type Hit%20Result%20Structure))
  (|CallParentFunction Other%20Actor HitResult)
  (bind _returnvalue (Game|SpawnActorfromClass "/Game/MagicGameMain/Blueprints/Systems/AOE/Bp_AOE_Fire.Bp_AOE_Fire_C" (Math|Transform|MakeTransform "0, 0, 0" "0, 0, 0" "1.000000,1.000000,1.000000") "Undefined" "MultiplyWithRoot" 0 1.0 5.0 false true false 0))
  (Utilities|FlowControl|Delay 0.2)
  (Actor|DestroyActor _returnvalue))

(fn ConstructionScript
  (|CallParentFunction))