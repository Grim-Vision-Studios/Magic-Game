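; BP_Pickup_Base is a parent Blueprint for pickups that are collected when a pawn touches them.
; Child Blueprints override GetPickupCollision to supply the collision component, whose begin overlap is bound on BeginPlay, with an on-screen error if it is missing.
; Pawn overlaps call Collected, an overridable event that by default plays CollectSound in 2D and destroys the actor.
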(event Custom|CollisionTouched
  (params (OverlappedComponent :type Primitive%20Component%20Object%20Reference) (OtherActor :type Actor%20Object%20Reference) (OtherComp :type Primitive%20Component%20Object%20Reference) (OtherBodyIndex :type Integer) (bFromSweep :type Boolean) (SweepResult :type Hit%20Result%20Structure%20%28by%20ref%29))
  ;[0 0 0] Checks if what overlaps pickup is a pawn.
  (bind _aspawn (Utilities|Casting|CastToPawn OtherActor))
  (CallFunction|Collected _aspawn))

(event Custom|Collected
  (params (Causer :type Pawn%20Object%20Reference))
  ;[0 0 0] Event Called When Pickup is collected, override in child BPs for specific functionality.
  (Audio|PlaySound2D (Variables|Pickup|GetCollectSound) 1.0 1.0 0.0 0 0)
  (Actor|DestroyActor))

(event EventBeginPlay
  (bind _pickup_collision (CallFunction|GetPickupCollision))
  (Utilities|IsValid _pickup_collision
    (:Is%20Valid
      (Collision|BindEventtoOnComponentBeginOverlap _pickup_collision (delegate Custom|CollisionTouched)))
    (:Is%20Not%20Valid
      (Development|PrintString (Utilities|String|Append (Utilities|GetDisplayName self) " does not have it's pickup collision set.") true true "(R=1.000000,G=0.000000,B=0.029831,A=1.000000)" 8.0))))

(fn ConstructionScript)

(fn GetPickupCollision
  (return 0))