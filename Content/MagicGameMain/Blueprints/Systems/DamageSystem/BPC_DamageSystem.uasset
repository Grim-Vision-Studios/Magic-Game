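; Damage system component that tracks an actor's health, death, invincibility, blocking and interruptibility.
; TakeDamage runs a damage info struct through CanBeDamage, which routes the hit to block, damage or no damage based on those states and the hit's override flags.
; It fires events for blocks (passing parry eligibility), death and interrupting hit responses, while Heal restores clamped health unless dead.
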(event EventBeginPlay)

(event EventTick
  (params (DeltaSeconds :type Float%20%28single-precision%29)))

(fn Heal
  (params (amount :type Float%20%28double-precision%29))
  (if (not (Variables|Default|GetIfDead))
    (bind _output_get (Variables|Default|SetHealth (Math|Float|Clamp(Float) (+ amount (Variables|Default|GetHealth)) 0.0 (Variables|Default|GetMaxHealth))))
    (return _output_get)))

(fn TakeDamage
  (params (DamageInfo :type S%20Info%20Structure))
  (bind (_amount _damagetype _damageresponse _shoulddamageinvincible _canbeblocked _canbeparried _shouldforceinterup) (Utilities|Struct|BreakS_Info DamageInfo))
  (Utilities|CanbeDamage _shoulddamageinvincible _canbeblocked
    (:BlockDamage
      (Default|CallOnBlocked _canbeparried)
      (return false))
    (:DoDamage
      (bind _output_get (Variables|Default|SetHealth (- (Variables|Default|GetHealth) _amount)))
      (if (<= _output_get 0.0)
        (Variables|Default|SetIfDead true)
        (Default|CallOnDeath)
        (return true)
        (elif (or (Variables|Default|GetIfInterruptible) _shouldforceinterup)
          (Default|CallOnDamageResponse _damageresponse)
          (return true))))
    (:NoDamage
      (return false))))