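; BP_AC_SkillHolder is a component that holds the equipped skill slots of its owning actor.
; On BeginPlay it constructs one empty BP_SkillObject per slot up to SkillNumber, outered to the owner and tagged with its index and a None skill tag.
; It stores them in EquippedSkills, fires an inventory-init call once they are built, and exposes the array through a getter.
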(event EventBeginPlay
  (CallFunction|InitSkillSlots))

(fn InitSkillSlots
  (for _index (range 0 (- (Variables|Default|GetSkillNumber) 1))
    (bind _returnvalue (Game|ConstructObjectfromClass (Components|GetOwner) "/Game/MagicGameMain/Blueprints/Skills/BP_SkillObject.BP_SkillObject_C" "None" _index))
    (Utilities|Array|Add (Variables|Default|GetEquippedSkills) _returnvalue))
  (Default|CallOnInventoryInit))

(fn GetEquippedSkills
  (return (Variables|Default|GetEquippedSkills)))