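; Lightning strike skill component that calls down a delayed area-of-effect attack on its target.
; On BeginPlay it caches its owning Pawn to serve as the instigator.
; StartUse spawns an AOE_LightingStrike at the target's location, passing the strike delay and target, and ignoring the instigator.
; The component binds to that actor's overlap event and sends a damage message to each actor reported.
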(event Custom|DamageEnemyAOE
  (params (Actor :type Actor%20Object%20Reference))
  (Class|BPIDamageInterface|TakeDamage(Message) Actor (Utilities|Struct|MakeS_Info (Variables|Default|GetDamage) "NewEnumerator3")))

(event EventBeginPlay
  (bind _aspawn (Utilities|Casting|CastToPawn (Components|GetOwner)))
  (Variables|Default|SetOwningPawn _aspawn))

(event EventTick
  (params (DeltaSeconds :type Float%20%28single-precision%29)))

(event EventStartUse
  (bind _target (Variables|Default|GetTarget))
  (bind _returnvalue (Game|SpawnActorfromClass "/Game/MagicGameMain/Blueprints/AOE/AOE_LightingStrike.AOE_LightingStrike_C" (Math|Transform|MakeTransform (Transformation|GetActorLocation _target) "0, 0, 0" "1.000000,1.000000,1.000000") "Undefined" "MultiplyWithRoot" (Components|GetOwner) (Variables|Default|GetStrikeDelay) _target true true false (Variables|Default|GetOwningPawn)))
  (EventDispatchers|BindEventtoOnAoeOverlapActor _returnvalue (delegate Custom|DamageEnemyAOE)))