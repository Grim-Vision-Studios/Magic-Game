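; Fire area-of-effect actor that overrides its parent's Trigger event to drop to the surface below and spawn a fire effect.
; After the parent logic, a debug-drawn Visibility trace runs from the actor to its location with Z multiplied by -1000.
; The actor moves to the hit location whether or not the trace hits, then attaches P_Fire to its root, passing that location.
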(event EventBeginPlay
  (|CallParentFunction) ; This node is disabled and will not be called.\nDrag off pins to build functionality.
)

(event Collision|EventActorBeginOverlap
  (params (OtherActor :type Actor%20Object%20Reference))
  (|CallParentFunction OtherActor) ; This node is disabled and will not be called.\nDrag off pins to build functionality.
)

(event EventTrigger
  (bind _returnvalue (Transformation|GetActorLocation))
  (|CallParentFunction)
  (bind (_outhit _returnvalue_2) (Collision|LineTraceByChannel _returnvalue (* _returnvalue "1.000000,1.000000,-1000.000000") "TraceTypeQuery1" false 0 "ForDuration"))
  (if _returnvalue_2
    _
    (else
      _))
  (Transformation|SetActorLocation (.Location (Collision|BreakHitResult _outhit)) false false)
  (Effects|SpawnEmitterAttached "/Game/StarterContent/Particles/P_Fire.P_Fire" (Variables|Default|GetDefaultSceneRoot) "None" (.Location (Collision|BreakHitResult _outhit))))

(fn ConstructionScript
  (|CallParentFunction))